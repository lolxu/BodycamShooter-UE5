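; First-person shooter player character that supplies procedural animation data through interface functions.
; A looping timer samples movement and mouse input into hand-sway floats, and the left-hand IK getter converts the weapon's LHIK socket into hand_r bone space.
; SetDOF applies camera depth of field at FocusLocation, and E spawns an enemy ahead.
; HeadBob is empty, with its speed-based camera-shake logic left disconnected.
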(event Custom|SetHandSwayFloats
  (Variables|Default|SetSide%20Movement (* (.x (Input|EnhancedActionValues|GetIA_Move)) (Variables|Default|GetSideMoveMultiplier)))
  (Variables|Default|SetMouse%20X (Class|Actor|GetInputAxisKeyValue))
  (Variables|Default|SetMouse%20Y (Class|Actor|GetInputAxisKeyValue)))

(event EventBeginPlay
  (Utilities|Time|SetTimerbyEvent (delegate Custom|SetHandSwayFloats) 0.015 true))

(event EventSetDOF
  ;[1 1 1] DOF
  (Variables|/Script/Engine.CameraComponent|SetPostProcessSettings (Variables|Default|GetCamera) (Utilities|Struct|MakePostProcessSettings 2.5 11.0 (Variables|Default|GetFocusLocation))))

(event EventHeadBob
  ;[1 1 1] HeadBob
)

(event Input|KeyboardEvents|E
  (params (Key :type Key%20Structure :default "None"))
  (bind _returnvalue (Transformation|GetActorLocation))
  (bind _returnvalue_2 (Transformation|GetActorForwardVector))
  (bind _spawnoffset (Variables|Default|GetSpawnOffset))
  (bind _returnvalue_3 (* _returnvalue_2 _spawnoffset))
  (bind _returnvalue_4 (+ _returnvalue _returnvalue_3))
  (bind _returnvalue_5 (Math|Rotator|FindLookatRotation _returnvalue _returnvalue_4))
  (bind (_roll _pitch _yaw) (Math|Rotator|BreakRotator _returnvalue_5))
  (:Pressed
    (Game|SpawnActorfromClass "/Game/BodyCam/Character/EnemyCharacter_BP.EnemyCharacter_BP_C" (Math|Transform|MakeTransform _returnvalue_4 (Math|Rotator|MakeRotator _roll _pitch (+ _yaw 9e+01))) "AdjustIfPossibleButAlwaysSpawn" "MultiplyWithRoot" 0 0)))

(fn ConstructionScript)

(fn IFGetHandSwayFloats
  (return (Variables|Default|GetSide%20Movement) (Variables|Default|GetMouse%20X) (Variables|Default|GetMouse%20Y)))

(fn IFGetLeftHandSocketTransform
  (bind _currentweapon (Variables|Default|GetCurrentWeapon))
  (bind _mesh (Variables|Character|GetMesh))
  (bind _mesh_2 (Variables|/Script/BodyCamShooter.Weapon|GetMesh _currentweapon))
  (bind _returnvalue (Transformation|GetSocketTransform _mesh_2 "LHIK" "RTS_World"))
  (bind (_outposition _outrotation) (Class|SkinnedMeshComponent|TransformtoBoneSpace _mesh "hand_r" (.location _returnvalue) (.rotation _returnvalue)))
  (Utilities|IsValid _currentweapon
    (:Is%20Valid
      (return (Math|Transform|MakeTransform _outposition _outrotation)))))