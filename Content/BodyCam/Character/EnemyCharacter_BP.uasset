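; Enemy character Blueprint that drives physical-animation hit reactions when the enemy is hit.
; While IsHit is set, Tick flags IsHitReacting and prints the hit bone name as debug output.
; It picks a reaction time by bone, much shorter for the head, and passes it with the hit result to PhysicalAnimComponent's HitReaction.
; IsHit is not cleared in these graphs, so the call repeats every frame while it stays true.
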(event EventBeginPlay)

(event Collision|EventActorBeginOverlap
  (params (OtherActor :type Actor%20Object%20Reference)))

(event EventTick
  (params (DeltaSeconds :type Float%20%28single-precision%29))
  (bind _enemyhitresult (Variables|Default|GetEnemyHitResult))
  (bind _hitbonename (Collision|BreakHitResult _enemyhitresult))
  (if (Variables|Default|GetbIsHit)
    (Variables|Default|SetIsHitReacting true)
    (Development|PrintString (Utilities|String|ToString(Name) _hitbonename))
    (switch name _hitbonename
      (:Default
        (Variables|Default|SetEnemyHitTime 1.35))
      (:head
        (Variables|Default|SetEnemyHitTime 0.1)))
    (Default|HitReaction (Variables|Default|GetPhysicalAnimComponent) (Variables|Default|GetEnemyHitResult) (Variables|Default|GetEnemyHitTime))))

(fn ConstructionScript)